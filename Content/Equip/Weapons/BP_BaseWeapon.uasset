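; BP_BaseWeapon is the base weapon Blueprint, a world pickup that can be attached to a player's mesh.
; When a pawn with an InventoryManager component overlaps its Box, the weapon sets that pawn as owner and adds itself to the inventory.
; AttachWeaponToCharacter casts the owner to Entity_Player and snaps the weapon to the named mesh socket, if that socket exists.
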(event `AttachWeaponToCharacter`
  (params (SocketName :type Name))
  (bind _asentity_player (cast `/Game/Blueprints/Entity_Player` (`self.GetOwner`)))
  (bind _mesh (`Character.Mesh` _asentity_player))
  (if (`SceneComponent.DoesSocketExist` _mesh SocketName)
    (`self.K2_AttachToComponent` _mesh SocketName "SnapToTarget" "SnapToTarget" "SnapToTarget")))

(event `self.Box.OnComponentBeginOverlap`
  (params (OverlappedComponent :type "PrimitiveComponent Object Reference") (OtherActor :type "Actor Object Reference") (OtherComp :type "PrimitiveComponent Object Reference") (OtherBodyIndex :type Integer) (bFromSweep :type Boolean) (SweepResult :type "HitResult Structure (by ref)"))
  (bind _aspawn (cast `Pawn` OtherActor))
  (bind _item (`KismetArrayLibrary.Array_Get` (`self.K2_GetComponentsByClass` _aspawn "/Game/Equip/InventoryManager.InventoryManager_C")))
  (`/Engine/EditorBlueprintResources/StandardMacros.IsValid` _item
    (:`Is Valid`
      (`self.SetOwner` OtherActor)
      (`/Game/Equip/InventoryManager.AddToInventory` _item self))))

(fn `UserConstructionScript`)