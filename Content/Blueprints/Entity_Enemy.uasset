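; Enemy character that patrols, chases and shoots the player, spawning its own AI controller and attaching a spawned weapon.
; Tick destroys it at zero health, otherwise runs an Idle, Target Spotted or Attacking state.
; AI Perception updates set the player as target and raise speed; random navmesh points drive patrol and chase.
; Attacking uses a line trace to fire, randomly returning to chase; older burst-fire logic is left unconnected.
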(event `self.ReceiveBeginPlay`
  (bind _returnvalue (`|SpawnActorFromClass` (`self.AIControllerClass`) (`KismetMathLibrary.MakeTransform` (0.0 0.0 0.0)) "AlwaysSpawn" "OverrideRootScale"))
  (`Controller.Possess` _returnvalue self)
  (bind _outactors (`GameplayStatics.GetAllActorsOfClass` "/Script/Engine.RecastNavMesh"))
  (set `self.NavData` (`KismetArrayLibrary.Array_Get` _outactors))
  (set `self.Health` 40.0))

(event `Spawn Weapon`
  (params (Class :type "Actor Class Reference"))
  (bind _returnvalue (`|SpawnActorFromClass` Class (`self.GetTransform`) "Undefined" "OverrideRootScale"))
  (bind _output_get (set `self.Weapon` (cast `/Game/Blueprints/Weapon_Base` _returnvalue :!pure true)))
  (`self.K2_AttachToComponent` _output_get (`self.CapsuleComponent`) "None" "SnapToTarget" "SnapToTarget" "KeepRelative" true))

(event `self.ReceiveTick`
  (params (DeltaSeconds :type "Float (single-precision)"))
  (bind _target (`self.Target`))
  (bind _target_2 (`self.Target`))
  (bind _weapon (`self.Weapon`))
  (`parent.ReceiveTick` DeltaSeconds)
  (if (<= (`self.Health`) 0.0)
    (`self.K2_DestroyActor`)
    (else
      (switch `/Game/Blueprints/AISTATE` (`self.State`)
        (:`NewEnumerator0`
          (if (not (`self.Moving`))
            (`|AIMoveTo` self (`NavigationSystem.GetRandomReachablePointInRadius` (`self.NavData`) (`self.K2_GetActorLocation`) 800.0)
              (:`then`
                (set `self.Moving` true))
              (:`OnSuccess`
                (`KismetSystemLibrary.Delay` (`KismetMathLibrary.RandomFloatInRange` 0.5 3.0) :!label _label)
                (set `self.Moving` false))
              (:`OnFail`
                (goto _label)))))
        (:`NewEnumerator1`
          (if (`self.Moving`)
            (`self.LookAt` _target)
            (else
              (`|AIMoveTo` self (`NavigationSystem.GetRandomReachablePointInRadius` (`self.K2_GetActorLocation` _target) 700.0 (`self.NavData`)) null 400.0
                (:`then`
                  (set `self.Moving` true))
                (:`OnSuccess`
                  (set `self.State` "NewEnumerator3")
                  (set `self.Moving` false))
                (:`OnFail`
                  (`KismetSystemLibrary.Delay` (`KismetMathLibrary.RandomFloatInRange` 1.0 3.0))
                  (set `self.Moving` false))))))
        (:`NewEnumerator3`
          (`self.LookAt` _target_2)
          (bind _outhit (`KismetSystemLibrary.LineTraceSingle` :`Start` (`self.K2_GetActorLocation`) :`End` (`self.K2_GetActorLocation` _target_2) :`TraceChannel` "TraceTypeQuery1" :`DrawDebugType` "ForOneFrame"))
          (bind (_bblockinghit _binitialoverlap _time _location _impactpoint _normal _impactnormal _physmat _hitactor) (`GameplayStatics.BreakHitResult` _outhit))
          (if _bblockinghit
            (cast `/Game/Blueprints/Entity_Player` _hitactor
              (:`then`
                (if (`self.Firing?`)
                  (if (== (`KismetMathLibrary.RandomIntegerInRange` 0 4) 1)
                    (set `self.Firing?` false)
                    (`/Game/Blueprints/Weapon_Base.Stop Attack` _weapon)
                    (set `self.State` "NewEnumerator1" :!label _label_2))
                  (else
                    (`/Game/Blueprints/Weapon_Base.Attack` _weapon)
                    (set `self.Firing?` true))))
              (:`CastFailed`
                (goto _label_2)))))))))

(event `self.AIPerception.OnPerceptionUpdated`
  (params (UpdatedActors :type "Array of Actor Object Reference"))
  (bind _item (`KismetArrayLibrary.Array_Get` UpdatedActors))
  (bind _info (`AIPerceptionComponent.GetActorsPerception` (`self.AIPerception`) _item))
  (set `self.Player Percieved` (`.bSuccessfullySensed` (break `AIStimulus` (`KismetArrayLibrary.Array_Get` (`.LastSensedStimuli` (break `ActorPerceptionBlueprintInfo` _info))))))
  (bind _asentity_player (cast `/Game/Blueprints/Entity_Player` _item))
  (set `self.Target` _asentity_player)
  (set `self.State` "NewEnumerator1")
  (set `self.Moving` false)
  (set `CharacterMovementComponent.MaxWalkSpeed` 500.0 (`self.CharacterMovement`)))

(fn `LookAt`
  (params (Target :type "Actor Object Reference"))
  (`self.K2_SetActorRotation` (`KismetMathLibrary.MakeRotator` 0.0 0.0 (.yaw (`KismetMathLibrary.FindLookAtRotation` (`self.K2_GetActorLocation`) (`self.K2_GetActorLocation` Target))))))

(fn `UserConstructionScript`
  (`parent.UserConstructionScript`))