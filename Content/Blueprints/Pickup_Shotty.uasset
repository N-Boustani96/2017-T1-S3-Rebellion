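; Shotgun pickup that arms an Entity_Player when the player overlaps it.
; If the player's Weapons array holds three or fewer entries, it spawns a Weapon_ShotGun, adds it to the array and snaps it to the player's root component.
; The new shotgun becomes the current weapon, then the pickup destroys itself and calls PickupPowerup on the player.
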(event `self.ReceiveActorBeginOverlap`
  (params (OtherActor :type "Actor Object Reference"))
  (bind _asentity_player (cast `/Game/Blueprints/Entity_Player` OtherActor))
  (bind _weapons (`/Game/Blueprints/Entity_Base.Weapons` _asentity_player))
  (if (<= (`KismetArrayLibrary.Array_Length` _weapons) 3)
    (bind _returnvalue (`|SpawnActorFromClass` "/Game/Blueprints/Weapon_ShotGun.Weapon_ShotGun_C" (`self.GetTransform` _asentity_player) "Undefined" "OverrideRootScale"))
    (`KismetArrayLibrary.Array_Add` _weapons _returnvalue)
    (`self.K2_AttachToComponent` _returnvalue (`self.K2_GetRootComponent` _asentity_player) "None" "SnapToTarget" "SnapToTarget" "SnapToTarget" false)
    (set `/Game/Blueprints/Entity_Base.CurrentWeapon` _returnvalue _asentity_player)
    (`self.K2_DestroyActor`)
    (`/Game/Blueprints/Entity_Player.PickupPowerup` _asentity_player)))

(fn `UserConstructionScript`
  (`parent.UserConstructionScript`))