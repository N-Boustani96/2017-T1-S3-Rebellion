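; Message_Printer is an interactable Blueprint that steps through a list of text messages on a TextRender component.
; Box overlap events toggle an InRange flag without checking which actor overlaps.
; Pressing Interact while in range calls ChangeText, which shows the next Messages entry, increments TextIndex and prints a debug "Hello".
; Once the index passes the last entry, further presses do nothing, as it never wraps or resets.
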(event `self.Box.OnComponentBeginOverlap`
  (params (OverlappedComponent :type "PrimitiveComponent Object Reference") (OtherActor :type "Actor Object Reference") (OtherComp :type "PrimitiveComponent Object Reference") (OtherBodyIndex :type Integer) (bFromSweep :type Boolean) (SweepResult :type "HitResult Structure (by ref)"))
  (set `self.inRange?` true))

(event `self.Box.OnComponentEndOverlap`
  (params (OverlappedComponent :type "PrimitiveComponent Object Reference") (OtherActor :type "Actor Object Reference") (OtherComp :type "PrimitiveComponent Object Reference") (OtherBodyIndex :type Integer))
  (set `self.inRange?` false))

(event `Change text`
  (bind _messages (`self.Messages`))
  (bind _textindex (`self.TextIndex`))
  (if (not (> _textindex (- (`KismetArrayLibrary.Array_Length` _messages) 1)))
    (`TextRenderComponent.K2_SetText` (`self.TextRender`) (`KismetTextLibrary.Conv_StringToText` (`KismetArrayLibrary.Array_Get` _messages _textindex)))
    (`/Engine/EditorBlueprintResources/StandardMacros.IncrementInt` _textindex
      (:`  `
        (`KismetSystemLibrary.PrintString` "Hello")))))

(event `InputAction|Interact` :consume false
  (params (Key :type "Key Structure" :default "AnyKey"))
  (:`Pressed`
    (if (`self.inRange?`)
      (`self.Change text`))))

(event `self.ReceiveBeginPlay`)

(fn `UserConstructionScript`)