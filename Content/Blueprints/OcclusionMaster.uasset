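; OcclusionMaster is an actor that trails the player and hides walls that overlap it, apparently to keep the player from being occluded.
; On BeginPlay it caches the first Entity_Player, then every Tick snaps to a fixed world-space offset from that player with a constant downward pitch.
; Overlap begin and end events cast the other actor to HideableWall and call HideWall or UnhideWall.
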(event `self.ReceiveBeginPlay`
  (bind _outactors (`GameplayStatics.GetAllActorsOfClass` "/Game/Blueprints/Entity_Player.Entity_Player_C"))
  (set `self.Player` (`KismetArrayLibrary.Array_Get` _outactors)))

(event `self.ReceiveTick`
  (params (DeltaSeconds :type "Float (single-precision)"))
  (`self.K2_SetActorTransform` (`KismetMathLibrary.MakeTransform` (+ (`self.K2_GetActorLocation` (`self.Player`)) (-247.0 0.0 302.0)) (`KismetMathLibrary.MakeRotator` 0.0 -50.0))))

(event `self.ReceiveActorBeginOverlap`
  (params (OtherActor :type "Actor Object Reference"))
  (bind _ashideable_wall (cast `/Game/Blueprints/HideableWall` OtherActor))
  (`/Game/Blueprints/HideableWall.Hide Wall` _ashideable_wall))

(event `self.ReceiveActorEndOverlap`
  (params (OtherActor :type "Actor Object Reference"))
  (bind _ashideable_wall (cast `/Game/Blueprints/HideableWall` OtherActor))
  (`/Game/Blueprints/HideableWall.Unhide Wall` _ashideable_wall))

(fn `UserConstructionScript`)