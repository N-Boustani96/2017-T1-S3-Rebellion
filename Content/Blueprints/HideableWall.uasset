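; HideableWall is a wall actor that fades to mostly transparent or back to opaque when HideWall or UnhideWall is called.
; BeginPlay puts a dynamic material instance on the static mesh, and the two events set opposing hide and show flags.
; While either flag is set, Tick steps the Opacity parameter through UpdateOpacity, clamped above zero.
; The flag-reset logic is disconnected, so updates continue after the fade finishes.
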(event `Unhide Wall`
  (if (`KismetSystemLibrary.IsValid` (`self.DynamicMaterial`))
    (set `self.Should Hide` false)
    (set `self.Should Show` true)))

(event `Hide Wall`
  (if (`KismetSystemLibrary.IsValid` (`self.DynamicMaterial`))
    (set `self.Should Hide` true)
    (set `self.Should Show` false)))

(event `self.ReceiveBeginPlay`
  (bind _staticmeshcomponent (`self.StaticMeshComponent`))
  (bind _returnvalue (`KismetMaterialLibrary.CreateDynamicMaterialInstance` (`PrimitiveComponent.GetMaterial` _staticmeshcomponent 0)))
  (bind _output_get (set `self.DynamicMaterial` _returnvalue))
  (`PrimitiveComponent.SetMaterial` _staticmeshcomponent 0 _output_get))

(event `self.ReceiveTick`
  (params (DeltaSeconds :type "Float (single-precision)"))
  (bind _should_hide (`self.Should Hide`))
  (if _should_hide
    (`self.Update Opacity` _should_hide (* DeltaSeconds 3.0) :!label _label)
    (elif (`self.Should Show`)
      (goto _label))))

(fn `Update Opacity`
  (params (Hiding :type Boolean) (Amount :type "Float (double-precision)"))
  (bind _dynamicmaterial (`self.DynamicMaterial`))
  (bind _returnvalue (`MaterialInstanceDynamic.K2_GetScalarParameterValue` _dynamicmaterial "Opacity"))
  (if Hiding
    (`MaterialInstanceDynamic.SetScalarParameterValue` _dynamicmaterial "Opacity" (`KismetMathLibrary.FClamp` (- _returnvalue Amount) 0.2))
    (else
      (`MaterialInstanceDynamic.SetScalarParameterValue` _dynamicmaterial "Opacity" (`KismetMathLibrary.FClamp` (+ _returnvalue Amount) 0.2)))))

(fn `UserConstructionScript`)