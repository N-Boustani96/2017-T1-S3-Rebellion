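; Entity_Base is an entity Blueprint, named as a base class, that provides health, death and a projectile attack.
; Attack spawns a TestBullet just ahead of the actor along its facing, passes it a fixed damage value, and plays a blaster sound.
; ApplyDamage subtracts from Health, while Tick polls that value and calls Die to destroy the actor once it reaches zero or below.
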(event `self.ReceiveTick`
  (params (DeltaSeconds :type "Float (single-precision)"))
  (if (<= (`self.Health`) 0.0)
    (`self.Die`)))

(fn `Apply Damage`
  (params (Value :type "Float (double-precision)"))
  (set `self.Health` (- (`self.Health`) Value)))

(fn `Attack`
  (bind _returnvalue (`self.K2_GetActorLocation`))
  (bind _returnvalue_2 (`self.K2_GetActorRotation`))
  (`|SpawnActorFromClass` "/Game/Blueprints/TestBullet.TestBullet_C" (`KismetMathLibrary.MakeTransform` (+ _returnvalue (* (`KismetMathLibrary.GetForwardVector` _returnvalue_2) 100.0)) _returnvalue_2) "Undefined" "OverrideRootScale" null 10.0)
  (`GameplayStatics.PlaySoundAtLocation` "/Game/Audio/Blaster_Sample.Blaster_Sample" _returnvalue))

(fn `Die`
  (`self.K2_DestroyActor`))

(fn `UserConstructionScript`)