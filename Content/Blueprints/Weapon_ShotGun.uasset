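; Shotgun weapon Blueprint that fires a three-projectile shot when its Attack event runs.
; Attack spawns one TestBullet actor at the world transform of each of three Arrow components, so their placement sets the spread.
; It then plays a blaster sound at the world origin rather than at the weapon's location.
; The construction script only calls the parent implementation.
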(event `self.Attack`
  (`|SpawnActorFromClass` "/Game/ThirdPersonBP/TestBullet.TestBullet_C" (`SceneComponent.K2_GetComponentToWorld` (`self.Arrow1`)) "Undefined" "OverrideRootScale")
  (`|SpawnActorFromClass` "/Game/ThirdPersonBP/TestBullet.TestBullet_C" (`SceneComponent.K2_GetComponentToWorld` (`self.Arrow`)) "Undefined" "OverrideRootScale")
  (`|SpawnActorFromClass` "/Game/ThirdPersonBP/TestBullet.TestBullet_C" (`SceneComponent.K2_GetComponentToWorld` (`self.Arrow2`)) "Undefined" "OverrideRootScale")
  (`GameplayStatics.PlaySoundAtLocation` "/Game/Audio/Blaster_Sample.Blaster_Sample"))

(fn `UserConstructionScript`
  (`parent.UserConstructionScript`))