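; Sniper weapon Blueprint that fires a projectile when its Attack event runs.
; Attack spawns a Projectile_Sniper just ahead of the actor along its facing direction, passes damage to it at spawn, and plays a blaster sound.
; A Cooling flag with a Delay blocks further shots until the cooldown ends.
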(event `self.Attack`
  (bind _returnvalue (`self.K2_GetActorLocation`))
  (bind _returnvalue_2 (`self.K2_GetActorRotation`))
  (if (not (`self.Cooling?`))
    (`|SpawnActorFromClass` "/Game/Blueprints/Projectile_Sniper.Projectile_Sniper_C" (`KismetMathLibrary.MakeTransform` (+ _returnvalue (* (`KismetMathLibrary.GetForwardVector` _returnvalue_2) 100.0)) _returnvalue_2) "Undefined" "OverrideRootScale" null 50.0)
    (`GameplayStatics.PlaySoundAtLocation` "/Game/Audio/Blaster_Sample.Blaster_Sample" _returnvalue)
    (set `self.Cooling?` true)
    (`KismetSystemLibrary.Delay` 3.0)
    (set `self.Cooling?` false)))

(fn `UserConstructionScript`
  (`parent.UserConstructionScript`))