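; Weapon_AR is an automatic weapon Blueprint that fires continuously between Attack and StopAttack calls.
; Attack fires immediately and starts a short looping timer that repeats Shoot, and StopAttack clears that timer.
; Each shot spawns a TestBullet just ahead of the weapon actor along its facing direction and plays a blaster sound at the actor's location.
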(event `self.Attack`
  (bind _returnvalue (`KismetSystemLibrary.K2_SetTimerDelegate` (delegate `Shoot`) 0.1 true))
  (set `self.Timer` _returnvalue)
  (`self.Shoot`))

(event `self.Stop Attack`
  (`KismetSystemLibrary.K2_ClearAndInvalidateTimerHandle` (`self.Timer`)))

(event `Shoot`
  (bind _returnvalue (`self.K2_GetActorLocation`))
  (bind _returnvalue_2 (`self.K2_GetActorRotation`))
  (`|SpawnActorFromClass` "/Game/ThirdPersonBP/TestBullet.TestBullet_C" (`KismetMathLibrary.MakeTransform` (+ _returnvalue (* (`KismetMathLibrary.GetForwardVector` _returnvalue_2) 100.0)) _returnvalue_2) "Undefined" "OverrideRootScale")
  (`GameplayStatics.PlaySoundAtLocation` "/Game/Audio/Blaster_Sample.Blaster_Sample" _returnvalue))

(fn `UserConstructionScript`
  (`parent.UserConstructionScript`))