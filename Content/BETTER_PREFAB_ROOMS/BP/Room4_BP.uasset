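; Room4_BP is a prefab room Blueprint that populates itself with enemies when play begins.
; BeginPlay rolls a small random enemy count, then loops, spawning a random class from the Enemies array at a random point inside the Box component's bounds.
; Spawns ignore collision, and each spawned actor's name and location are printed on screen as debug output.
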(event `self.ReceiveBeginPlay`
  (bind _enemies (`self.Enemies`))
  (bind _box (`self.Box`))
  (set `self.NumberofEnemies` (`KismetMathLibrary.RandomIntegerInRange` 1 4))
  (while (not (>= (`self.Spawncount`) (`self.NumberofEnemies`)))
    (bind _returnvalue (`|SpawnActorFromClass` (`KismetArrayLibrary.Array_Get` _enemies (`KismetMathLibrary.RandomIntegerInRange` 0 (- (`KismetArrayLibrary.Array_Length` _enemies) 1))) (`KismetMathLibrary.MakeTransform` (`KismetMathLibrary.RandomPointInBoundingBox` (`SceneComponent.K2_GetComponentLocation` _box) (`BoxComponent.GetScaledBoxExtent` _box))) "AlwaysSpawn" "OverrideRootScale"))
    (set `self.Spawncount` (+ (`self.Spawncount`) 1))
    (`KismetSystemLibrary.PrintString` (`KismetSystemLibrary.GetObjectName` _returnvalue) true true (struct :`G` 0.66 :`B` 1.0 :`A` 1.0) 20.0)
    (`KismetSystemLibrary.PrintString` (`KismetStringLibrary.Conv_VectorToString` (`self.K2_GetActorLocation` _returnvalue)) true true (struct :`G` 1.0 :`B` 0.10461 :`A` 1.0) 20.0)))

(fn `UserConstructionScript`)